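; Strategy-style turn manager for a turn-based tactics game, extending a parent manager so that turns run per faction.
; Faction turn start notifies the faction's actors, deselects the active one, sets the owning player to the Idle ability and auto-selects AI-controlled units.
; After each ability, unexhausted actors are reselected, while exhausted AI advances to the next actor and players return to Idle.
; The faction turn ends on player input or when no refreshed actors remain.
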(event `self.BeginActiveFactionTurn`
  (bind _activeplayer (`self.ActivePlayer`))
  ;[0 1 0.6948] Begin Active Faction Turn
  (bind _actorsoffaction (`self.FindInitiativeActorsOfFaction` (`self.ActiveFaction`)))
  (for _array_element _actorsoffaction
    (message `/Game/AdvancedTurnBasedTileToolkit/Core/BPI_Initiative.RunOnBeginActorTurn` _array_element))
  (message `/Game/AdvancedTurnBasedTileToolkit/Core/BPI_Initiative.DeselectActor` (`self.ActiveActor`))
  (bind (_bfoundvalidactor _actor) (`self.FindNextRefreshedActor`))
  (if _bfoundvalidactor
    (bind _asbp_player_controller_atbtt (cast `/Game/AdvancedTurnBasedTileToolkit/Core/BP_PlayerController_ATBTT` (`self.GetOwner` _actor))
      (:`then`
        (set `self.ActivePlayer` _asbp_player_controller_atbtt)
        (message `/Game/AdvancedTurnBasedTileToolkit/Core/BPI_PC.ActivateAbility` _activeplayer "/Game/AdvancedTurnBasedTileToolkit/Core/Abilities/BP_AbilityBase_Idle.BP_AbilityBase_Idle_C" _activeplayer))
      (:`CastFailed`
        (set `self.ActivePlayer` null)))
    (`self.QueueDisplayFactionTurn`)
    (bind _baicontrolled (message `/Game/AdvancedTurnBasedTileToolkit/Core/BPI_Initiative.GetAiControlled` _actor))
    (if _baicontrolled
      (message `/Game/AdvancedTurnBasedTileToolkit/Core/BPI_Initiative.SelectActor` _actor))
    (else
      (`self.EndActiveFactionTurn`))))

(event `self.RunAfterAbilityExecute`
  (bind _activeactor (`self.ActiveActor`))
  (bind _activeplayer (`self.ActivePlayer`))
  ;[0.4688 0 0.3991] Run After Ability Execute
  (bind _bexhausted (message `/Game/AdvancedTurnBasedTileToolkit/Core/BPI_Initiative.CheckIfExhausted` (`self.ActiveActor`)))
  (if _bexhausted
    (bind _baicontrolled (message `/Game/AdvancedTurnBasedTileToolkit/Core/BPI_Initiative.GetAiControlled` _activeactor))
    (if _baicontrolled
      (`self.BeginNextValidActorTurn` false)
      (else
        (bind _bfoundvalidactor (`self.FindNextRefreshedActor`))
        (if _bfoundvalidactor
          (message `/Game/AdvancedTurnBasedTileToolkit/Core/BPI_PC.ActivateAbility` _activeplayer "/Game/AdvancedTurnBasedTileToolkit/Core/Abilities/BP_AbilityBase_Idle.BP_AbilityBase_Idle_C" _activeplayer)
          (else
            (`self.EndActiveFactionTurn`)))))
    (else
      (message `/Game/AdvancedTurnBasedTileToolkit/Core/BPI_Initiative.SelectActor` _activeactor))))

(event `self.EndTurnFromPlayerInput`
  ;[1 0.954 0] EndTurnFromPlayerInput
  (`self.EndActiveFactionTurn`))

(fn `UserConstructionScript`
  (`parent.UserConstructionScript`))