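; BP_MazeGrid is an actor that builds a seeded grid maze in its Construction Script, placing a HierarchicalInstancedStaticMesh instance on each path tile.
; GenerateMaze carves with randomized depth-first search, recursing through AddNeighborLoc in two-cell steps and recording the bridge cell between them.
; When stuck, Backtrack pops the last pending cell and moves a bridge into the path set.
; Dead ends are collected in EndPaths, which construction leaves unused.
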(fn `AddNeighborLoc`
  (params (Size :type "IntPoint Structure (by ref)") (RandStream :type "RandomStream Structure (by ref)") (CurrentLc :type "IntPoint Structure (by ref)") (PathTiles :type "Set of IntPoint Structure (by ref)") (BridgeTiles :type "Set of IntPoint Structure (by ref)") (ToCheck :type "Set of IntPoint Structure (by ref)") (EndPaths :type "Set of IntPoint Structure (by ref)"))
  (locals (NeighborIndex :type Integer))
  (bind _returnvalue (+ (`local.NeighborIndex`) 1))
  (bind (_floor _bridge) (`self.GetNeighborAndBridge` (`local.CurrentLc`) (`local.NeighborIndex`)))
  (set `local.NeighborIndex` (`KismetMathLibrary.RandomIntegerInRangeFromStream` 0 3 (`local.RandStream`)))
  (if (`self.CheckIsValidLoc` (`self.GetNeighborAndBridge` (`local.CurrentLc`) (`local.NeighborIndex`)) (`self.Size`) (`local.PathTiles`) (`local.BridgeTiles`)) :!label _label
    (`BlueprintSetLibrary.Set_Add` (`local.PathTiles`) _floor)
    (`BlueprintSetLibrary.Set_Add` (`local.BridgeTiles`) _bridge)
    (`BlueprintSetLibrary.Set_Add` (`local.ToCheck`) _floor)
    (`self.AddNeighborLoc` (`local.Size`) (`local.RandStream`) _floor (`local.PathTiles`) (`local.BridgeTiles`) (`local.ToCheck`) (`local.EndPaths`))
    (else
      (`/Game/ParentBlueprints/Custom_Mac_Library.DoN+` 4
        (:`Exit`
          (set `local.NeighborIndex` (`KismetMathLibrary.SelectInt` 0 _returnvalue (>= _returnvalue 4)))
          (goto _label))
        (:`OverNth`
          (bind _count (`self.GetNeighborCount` (`local.CurrentLc`) (`local.PathTiles`)))
          (if (== _count 1)
            (`BlueprintSetLibrary.Set_Add` (`local.EndPaths`) (`local.CurrentLc`))))))))

(fn `Backtrack`
  (params (CurrentTile :type "IntPoint Structure (by ref)") (ToCheck :type "Set of IntPoint Structure (by ref)") (PathTiles :type "Set of IntPoint Structure (by ref)") (BridgeTiles :type "Set of IntPoint Structure (by ref)"))
  (bind _result (`BlueprintSetLibrary.Set_ToArray` ToCheck))
  (bind _output (`|GetArrayItem` _result (`KismetArrayLibrary.Array_LastIndex` _result)))
  (`|VariableSetRef` (`local.CurrentTile`) _output)
  (`BlueprintSetLibrary.Set_Remove` (`local.ToCheck`) _output)
  (bind _result_2 (`BlueprintSetLibrary.Set_ToArray` (`local.BridgeTiles`)))
  (bind _output_2 (`|GetArrayItem` _result_2 (`KismetArrayLibrary.Array_LastIndex` _result_2)))
  (`BlueprintSetLibrary.Set_Add` (`local.PathTiles`) _output_2)
  (`BlueprintSetLibrary.Set_Remove` (`local.BridgeTiles`) _output_2))

(fn `GenerateMaze`
  (params (Seed :type "Integer (by ref)") (Size :type "IntPoint Structure (by ref)"))
  (returns (PathTiles_Out :type "Set of IntPoint Structure") (EndPaths_OUt :type "Set of IntPoint Structure"))
  (locals (RandStream :type "RandomStream Structure") (L_Size :type "IntPoint Structure") (StartingLc :type "IntPoint Structure") (CurrentLc :type "IntPoint Structure") (PathTiles :type "Set of IntPoint Structure") (BridgeTiles :type "Set of IntPoint Structure") (ToCheck :type "Set of IntPoint Structure") (EndPaths :type "Set of IntPoint Structure"))
  (`KismetMathLibrary.SetRandomStreamSeed` (`local.RandStream`) Seed)
  (set `local.L_Size` Size)
  (bind _output_get (set `local.StartingLc` (`self.GetRandLocInBounds` (`local.L_Size`) (`local.RandStream`))))
  (set `local.CurrentLc` _output_get)
  (`self.AddNeighborLoc` (`local.L_Size`) (`local.RandStream`) (`local.CurrentLc`) (`local.PathTiles`) (`local.BridgeTiles`) (`local.ToCheck`) (`local.EndPaths`) :!label _label)
  (if (> (`BlueprintSetLibrary.Set_Length` (`local.ToCheck`)) 0)
    (`self.Backtrack` (`local.CurrentLc`) (`local.ToCheck`) (`local.PathTiles`) (`local.BridgeTiles`))
    (goto _label)
    (else
      (return (`local.PathTiles`) (`local.EndPaths`)))))

(fn `GetNeighborCount`
  (params (CurrentLc :type "IntPoint Structure (by ref)") (PathTiles :type "Set of IntPoint Structure (by ref)"))
  (returns (Count :type Integer))
  (locals (Counter :type Integer))
  (for _array_element (`self.GetNeighborLoc` (struct) 1)
    (if (`BlueprintSetLibrary.Set_Contains` (`local.PathTiles`) _array_element)
      (`/Engine/EditorBlueprintResources/StandardMacros.IncrementInt` (`local.Counter`))))
  (return (`local.Counter`)))

(fn `UserConstructionScript`
  (bind _tilesize (`self.TileSize`))
  (bind _pathtiles_out (`self.GenerateMaze` (`self.Seed`) (`self.Size`)))
  (bind _result (`BlueprintSetLibrary.Set_ToArray` _pathtiles_out))
  (for _array_element _result
    (bind (_x _y) (break `IntPoint` _array_element))
    (`InstancedStaticMeshComponent.AddInstance` (`self.HierarchicalInstancedStaticMesh`) (`KismetMathLibrary.MakeTransform` (`KismetMathLibrary.MakeVector` (* _x _tilesize) (* _y _tilesize))))))